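; Blackjack game controller that builds the board widget, player pawns and card deck, with the last pawn as dealer.
; StartGame shuffles and deals two cards each, hiding the dealer's second.
; Turns pass by possessing each pawn in order, with hit and stand arriving through an interface, until the dealer plays automatically.
; DealerEnds compares scores against the dealer's, treating non-positive scores as bust, and updates the UI with results.
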(event Custom|Create%20Card%20Deck
  ;[1 0.04985 0.6496] Spawn cards, assign their values then shuffle the deck
  (for _index (range 0 3)
    (for _index_2 (range 2 10)
      (CallFunction|SpawnCard _index_2 (Utilities|String|ToString(Integer) _index_2)))
    (bind _returnvalue (Class|DataTableFunctionLibrary|GetDataTableColumnasString (Variables|Default|GetDT_Deck) "CardName"))
    (for _array_element _returnvalue
      (if (Utilities|Enum|Equal(Enum) _array_element "A")
        (bind _returnvalue_2 (Game|SpawnActorfromClass "/Game/BlackJack_bp/BP_Card_Ace.BP_Card_Ace_C" (Math|Transform|MakeTransform "0, 0, 0" "0, 0, 0" "1.000000,1.000000,1.000000") "Undefined" "MultiplyWithRoot" 0 0))
        (Utilities|Array|Add (Variables|Default|GetCardDeck) _returnvalue_2)
        (else
          (CallFunction|SpawnCard 10 _array_element))))))

(event Custom|Deal%20Cards
  ;[0 0.319 1] Comment
  (for _index (range 0 1)
    (for _array_element (Variables|Default|GetPlayerList)
      (if (and (Variables|/Game/BlackJack_bp/BP_BlackJack_Pawn.BP_BlackJack_Pawn_C|GetIsDealer _array_element) (== _index 1))
        (Default|AddCardtoHand _array_element (Utilities|Array|Get(acopy) (Variables|Default|GetCardDeck) (Variables|Default|GetCurrent%20Card)) false)
        (Math|Integer|IncrementInt (Variables|Default|GetCurrent%20Card))
        (else
          (Default|AddCardtoHand _array_element (Utilities|Array|Get(acopy) (Variables|Default|GetCardDeck) (Variables|Default|GetCurrent%20Card)) true)
          (Math|Integer|IncrementInt (Variables|Default|GetCurrent%20Card)))))))

(event EventBeginPlay
  ;[1 0 0.245] Comment
  (CallFunction|IntiializeGame))

(event EventPlayerEndTurn
  (params (Player%20Pawn :type Pawn%20Object%20Reference))
  (bind _current_player_index (Variables|Default|GetCurrent%20Player%20Index))
  ;[1 1 1] BPI Player Interaction Implementation
  ;;[0.7457 0 1] Comment
  (if (not (== (Variables|Default|GetDealerPlayer) Player%20Pawn))
    (if (not (== (Variables|Default|GetNumPlayers) _current_player_index))
      (bind _result (Math|Integer|IncrementInt _current_player_index)
        (:%20%20
          (Variables|Default|SetCurrent%20Player (Utilities|Array|Get(acopy) (Variables|Default|GetPlayerList) _result))
          (if (== (Variables|Default|GetCurrent%20Player) (Variables|Default|GetDealerPlayer))
            (Development|PrintString "Dealer is now playing")
            (Default|DealerPlay (Variables|Default|GetCurrent%20Player))
            (else
              (bind _current_player (Variables|Default|GetCurrent%20Player)
                (:then
                  (Pawn|Possess (Game|GetPlayerController 0) _current_player)
                  (Default|PlayerBeginTurn _current_player))
                (:else
                  (Development|PrintString "Not valid" true true "(R=0.942751,G=0.000000,B=1.000000,A=1.000000)"))))))))))

(event EventDealerEnds
  ;[1 1 1] BPI Player Interaction Implementation
  ;;[0.8948 0 1] Comment
  (Development|PrintString "-----The game ends-----")
  (Development|PrintString (Utilities|String|Append "The dealer finishes with a score of " (Utilities|String|ToString(Integer) (Variables|/Game/BlackJack_bp/BP_BlackJack_Pawn.BP_BlackJack_Pawn_C|GetPlayer%20Score (Variables|Default|GetDealerPlayer)))))
  (CallFunction|DetermineWinners)
  (for _array_element (Variables|Default|GetPlayerList)
    (if (not (== (Variables|Default|GetDealerPlayer) _array_element))
      (Development|PrintString (Utilities|String|Append (Variables|/Game/BlackJack_bp/BP_BlackJack_Pawn.BP_BlackJack_Pawn_C|GetPlayerName _array_element) " " (Variables|/Game/BlackJack_bp/BP_BlackJack_Pawn.BP_BlackJack_Pawn_C|GetPlayer%20Status _array_element)))))
  (Development|PrintString "The game ends")
  (Default|GameEnds (Variables|Default|GetBlackjack%20Widget%20Main)))

(event EventStartGame
  ;[1 1 1] BPI Player Interaction Implementation
  ;;[0.01656 0 1] Comment
  (Variables|Default|SetCurrent%20Card 0)
  ;;;[1 0 0.3151] Comment
  (Default|CallDiscardHand)
  (Utilities|Array|Shuffle (Variables|Default|GetCardDeck))
  (CallFunction|DealCards)
  (Variables|Default|SetCurrent%20Player%20Index -1)
  ;;;[1 1 1] Next player begin turn
  (CallFunction|PlayerEndTurn))

(event EventPlayerStand
  ;[1 1 1] BPI Player Interaction Implementation
  ;;[0 0.1624 1] Comment
  (CallFunction|PlayerEndTurn (Variables|Default|GetCurrent%20Player)))

(event EventPlayerHit
  ;[1 1 1] BPI Player Interaction Implementation
  ;;[0 0.1111 1] Comment
  (Default|AddCardtoHand (Variables|Default|GetCurrent%20Player) (Utilities|Array|Get(acopy) (Variables|Default|GetCardDeck) (Variables|Default|GetCurrent%20Card)) true)
  (Math|Integer|IncrementInt (Variables|Default|GetCurrent%20Card)))

(fn ConstructionScript)

(fn SpawnCard
  (params (Card%20Value :type Integer) (CardName :type String))
  (bind _returnvalue (Game|SpawnActorfromClass "/Game/BlackJack_bp/BP_Card.BP_Card_C" (Math|Transform|MakeTransform "0, 0, 0" "0, 0, 0" "1.000000,1.000000,1.000000") "Undefined" "MultiplyWithRoot" 0 0))
  (Default|SetupCard _returnvalue Card%20Value CardName)
  (Utilities|Array|Add (Variables|Default|GetCardDeck) _returnvalue))

(fn DetermineWinners
  ;[0.6951 0 1] Comment
  (LocalVariables|SetDealer%20Score (Variables|/Game/BlackJack_bp/BP_BlackJack_Pawn.BP_BlackJack_Pawn_C|GetPlayer%20Score (Variables|Default|GetDealerPlayer)))
  (for _array_element (Variables|Default|GetPlayerList)
    (LocalVariables|SetLocalCurrentPlayer _array_element)
    (bind _output_get (LocalVariables|SetCurrent%20Player%20Score (Variables|/Game/BlackJack_bp/BP_BlackJack_Pawn.BP_BlackJack_Pawn_C|GetPlayer%20Score _array_element)))
    (if (> _output_get 0)
      (if (> (LocalVariables|GetCurrent%20Player%20Score) (LocalVariables|GetDealer%20Score))
        (Variables|/Game/BlackJack_bp/BP_BlackJack_Pawn.BP_BlackJack_Pawn_C|SetPlayer%20Status (LocalVariables|GetLocalCurrentPlayer) (Utilities|String|Append "Wins with a score of  " (Utilities|String|ToString(Integer) (Variables|/Game/BlackJack_bp/BP_BlackJack_Pawn.BP_BlackJack_Pawn_C|GetPlayer%20Score (LocalVariables|GetLocalCurrentPlayer)))))
        (Default|UpdatePlayerStatus (Variables|/Game/BlackJack_bp/BP_BlackJack_Pawn.BP_BlackJack_Pawn_C|GetPlayer%20Hand%20Widget (LocalVariables|GetLocalCurrentPlayer)) "Winner!")
        (elif (== (LocalVariables|GetCurrent%20Player%20Score) (LocalVariables|GetDealer%20Score))
          (Variables|/Game/BlackJack_bp/BP_BlackJack_Pawn.BP_BlackJack_Pawn_C|SetPlayer%20Status (LocalVariables|GetLocalCurrentPlayer) "Ties with the dealer")
          (Default|UpdatePlayerStatus (Variables|/Game/BlackJack_bp/BP_BlackJack_Pawn.BP_BlackJack_Pawn_C|GetPlayer%20Hand%20Widget (LocalVariables|GetLocalCurrentPlayer)) "Tie")
          (else
            (Variables|/Game/BlackJack_bp/BP_BlackJack_Pawn.BP_BlackJack_Pawn_C|SetPlayer%20Status (LocalVariables|GetLocalCurrentPlayer) "Loses to dealer")
            (Default|UpdatePlayerStatus (Variables|/Game/BlackJack_bp/BP_BlackJack_Pawn.BP_BlackJack_Pawn_C|GetPlayer%20Hand%20Widget (LocalVariables|GetLocalCurrentPlayer)) "Loser"))))
      (else
        (Variables|/Game/BlackJack_bp/BP_BlackJack_Pawn.BP_BlackJack_Pawn_C|SetPlayer%20Status (LocalVariables|GetLocalCurrentPlayer) "is Bust")))))

(fn IntiializeGame
  ;[0.5849 0 1] Setup Players
  (Utilities|FlowControl|Sequence
    (:then_0
      ;;[0 0.1506 1] Create UI Widget
      (bind _returnvalue (UserInterface|CreateWidget "/Game/Widgets/WBP_BlackJackBoard.WBP_BlackJackBoard_C"))
      (bind _output_get (Variables|Default|SetBlackjack%20Widget%20Main _returnvalue))
      (UserInterface|Viewport|AddtoViewport _output_get 0))
    (:then_1
      (for _index (range 0 (Variables|Default|GetNumPlayers))
        (bind _returnvalue_2 (Game|SpawnActorfromClass "/Game/BlackJack_bp/BP_BlackJack_Pawn.BP_BlackJack_Pawn_C" (Math|Transform|MakeTransform "0, 0, 0") "Undefined" "MultiplyWithRoot" 0 0))
        (bind _output_get_2 (LocalVariables|SetNew%20Pawn _returnvalue_2))
        (Utilities|Array|Add (Variables|Default|GetPlayerList) _output_get_2)
        ;;[1 1 1] Set last player to dealer
        (if (== _index (Variables|Default|GetNumPlayers))
          (Variables|/Game/BlackJack_bp/BP_BlackJack_Pawn.BP_BlackJack_Pawn_C|SetIsDealer (LocalVariables|GetNew%20Pawn) true)
          (Variables|/Game/BlackJack_bp/BP_BlackJack_Pawn.BP_BlackJack_Pawn_C|SetPlayerName (LocalVariables|GetNew%20Pawn) "Dealer")
          (Variables|Default|SetDealerPlayer (LocalVariables|GetNew%20Pawn))
          (else
            (Variables|/Game/BlackJack_bp/BP_BlackJack_Pawn.BP_BlackJack_Pawn_C|SetPlayerName (LocalVariables|GetNew%20Pawn) (Utilities|String|Append "Player " (Utilities|String|ToString(Integer) _index)))))))
    (:then_2
      (CallFunction|CreateCardDeck)
      (Default|CreateHandforPlayers (Variables|Default|GetBlackjack%20Widget%20Main) (Variables|Default|GetPlayerList)))))