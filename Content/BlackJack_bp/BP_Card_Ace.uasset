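; BP_Card_Ace is the Ace card Blueprint for a blackjack game, a child card that can drop its value to 1.
; AceReduceValue sets CardValue to 1, prints a debug message with the card name, and returns true, or returns false if the value is already 1.
; The construction script only calls the parent version.
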(fn ConstructionScript
  (|CallParentFunction))

(fn AceReduceValue
  (if (== (Variables|Default|GetCardValue) 1)
    (return false)
    (else
      (Variables|Default|SetCardValue 1)
      (Development|PrintString (Utilities|String|Append (Utilities|GetDisplayName self) " " (Variables|Default|GetCardName) " Reduced to 1"))
      (return true))))