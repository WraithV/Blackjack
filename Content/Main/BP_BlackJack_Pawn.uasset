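; Blackjack pawn for a player or the dealer, holding a hand of cards, its score and a WBP_PlayerHand widget.
; Face-up cards trigger scoring, which lowers aces while over WinScore, then auto-stands on WinScore or busts.
; Turn ends are reported to the game mode, whose discard event clears the hand.
; As dealer, it flips its hidden card and requests hits in a bounded loop until reaching DealerMin or finishing.
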(event Custom|Add%20Card%20to%20Hand
  (params (New%20Card :type BP%20Card%20Object%20Reference) (FaceUp? :type Boolean))
  (bind _cardname (Variables|/Game/Main/BP_Card.BP_Card_C|GetCardName New%20Card))
  ;[0 0.3185 1] Add card to hand and create widget for this card, if it is face down don't add its value to the players total
  (Utilities|Array|Add (Variables|Default|GetPlayerHand) New%20Card)
  (Default|AddCard (Variables|Default|GetPlayer%20Hand%20Widget) _cardname FaceUp?)
  (if FaceUp?
    (CallFunction|CalculatePlayerScore)
    (Development|PrintString (Utilities|String|Append (Variables|Default|GetPlayerName) " Pulls a " _cardname) true true "(R=1.000000,G=0.429715,B=0.000000,A=1.000000)")))

(event Custom|Player%20Bust
  ;[1 1 1] Player is Bust update status, score and end turn
  (Default|UpdatePlayerStatus (Variables|Default|GetPlayer%20Hand%20Widget) "BUST!!")
  (Variables|Default|SetPlayer%20Score -1)
  (Class|BPIPlayerActions|PlayerEndTurn(Message) (Game|GetGameMode) self))

(event Custom|Player%20Stand
  (Default|UpdatePlayerStatus (Variables|Default|GetPlayer%20Hand%20Widget) "Stand")
  (Class|BPIPlayerActions|PlayerEndTurn(Message) (Game|GetGameMode) self))

(event Custom|Dealer%20Play
  ;[1 1 1] Only if player is Dealer
  (CallFunction|FlipCard)
  (bind _continue (CallFunction|CalculatePlayerScore))
  (if _continue
    (if (>= (Variables|Default|GetPlayer%20Score) (Variables|Default|GetDealer%20Min))
      (CallFunction|PlayerStand)
      (Class|BPIPlayerActions|DealerEnds(Message) (Game|GetGameMode))
      (else
        (Utilities|FlowControl|ForLoopwithBreak 0 10 :!label _label
          (:LoopBody
            (Class|BPIPlayerActions|PlayerHit(Message) (Game|GetGameMode))
            (bind _continue_2 (CallFunction|CalculatePlayerScore))
            (if (or (not _continue_2) (>= (Variables|Default|GetPlayer%20Score) (Variables|Default|GetDealer%20Min)))
              (goto _label Break)))
          (:Completed
            (Class|BPIPlayerActions|DealerEnds(Message) (Game|GetGameMode))))))
    (else
      (Class|BPIPlayerActions|DealerEnds(Message) (Game|GetGameMode)))))

(event Custom|Flip%20Card
  ;[1 1 1] Only if player is Dealer
  ;;[1 1 1] Flip 2nd card - need to trigger reveal
  (Default|FlipCards (Variables|Default|GetPlayer%20Hand%20Widget))
  (Development|PrintString (Utilities|String|Append "Dealers current score is  " (Utilities|String|ToString(Integer) (Variables|Default|GetPlayer%20Score)) " Till he flips...")))

(event Custom|Player%20Begin%20Turn
  ;[1 1 1] Just updates player status
  (Default|UpdatePlayerStatus (Variables|Default|GetPlayer%20Hand%20Widget) "Playing")
  (Development|PrintString (Utilities|String|Append "Now playing " (Variables|Default|GetPlayerName) " with a score of " (Utilities|String|ToString(Integer) (Variables|Default|GetPlayer%20Score)))))

(event Custom|Create%20Player%20Hand
  ;[1 1 1] Create hand widget and setup variables
  (bind _returnvalue (UserInterface|CreateWidget "/Game/Widgets/WBP_PlayerHand.WBP_PlayerHand_C"))
  (bind _output_get (Variables|Default|SetPlayer%20Hand%20Widget _returnvalue))
  (Default|UpdatePlayerName _output_get (Variables|Default|GetPlayerName))
  (Default|UpdatePlayerScore _output_get (Variables|Default|GetPlayer%20Score))
  (Default|UpdatePlayerStatus _output_get (Variables|Default|GetPlayer%20Status)))

(event Custom|Discard%20Cards
  ;[0 0.2597 1] Reset player hand and remove card widgets
  (Variables|Default|SetPlayer%20Score 0)
  (Utilities|Array|Clear (Variables|Default|GetPlayerHand))
  (Default|WidgetResetHand (Variables|Default|GetPlayer%20Hand%20Widget)))

(event EventBeginPlay
  ;[1 0.2958 0.3856] Comment
  (bind _asblack_jack_game_mode (Utilities|Casting|CastToBlackJack_GameMode (Game|GetGameMode)))
  (EventDispatchers|BindEventtoDiscardHand _asblack_jack_game_mode (delegate Custom|Discard%20Cards)))

(fn ConstructionScript)

(fn CalculatePlayerScore
  ;[0 0.2074 1] Comment
  (Utilities|FlowControl|Sequence
    (:then_0
      ;[1 1 1] Add up non ace card values, add ace cards to temporary array
      (for _array_element (Variables|Default|GetPlayerHand)
        (bind _output_get (LocalVariables|SetCurrentCard _array_element))
        (bind _asbp_card_ace (Utilities|Casting|CastToBP_Card_Ace (LocalVariables|GetCurrentCard))
          (:then
            (Utilities|Array|Add (LocalVariables|GetAceArray) _asbp_card_ace)
            (LocalVariables|SetAceValues (+ (LocalVariables|GetAceValues) (Variables|/Game/Main/BP_Card.BP_Card_C|GetCardValue _asbp_card_ace))))
          (:CastFailed
            (LocalVariables|SetcurrentScore (+ (LocalVariables|GetcurrentScore) (Variables|/Game/Main/BP_Card.BP_Card_C|GetCardValue _output_get))))))
      (Development|PrintString (Utilities|String|Append "Ace values " (Utilities|String|ToString(Integer) (LocalVariables|GetAceValues)))))
    (:then_1
      ;[1 1 1] Reduce value of aces until card value is less than 21 then break
      (if (> (+ (LocalVariables|GetcurrentScore) (LocalVariables|GetAceValues)) (Variables|Default|GetWinScore))
        (bind _array_element_2 (Utilities|Array|ForEachLoopwithBreak (LocalVariables|GetAceArray) :!label _label)
          (:LoopBody
            (bind _reduced (Default|AceReduceValue _array_element_2))
            (if _reduced
              (LocalVariables|SetAceValues (- (LocalVariables|GetAceValues) 10)))
            (if (not (> (+ (LocalVariables|GetcurrentScore) (LocalVariables|GetAceValues)) (Variables|Default|GetWinScore)))
              (goto _label Break)))
          (:Completed
            (Development|PrintString (Utilities|String|Append "Final ace values = " (Utilities|String|ToString(Integer) (LocalVariables|GetAceValues))))))))
    (:then_2
      (bind _output_get_2 (Variables|Default|SetPlayer%20Score (+ (LocalVariables|GetcurrentScore) (LocalVariables|GetAceValues))))
      (Default|UpdatePlayerScore (Variables|Default|GetPlayer%20Hand%20Widget) _output_get_2)
      (if (> _output_get_2 (Variables|Default|GetWinScore))
        (CallFunction|PlayerBust)
        (return false)
        (elif (== (Variables|Default|GetPlayer%20Score) (Variables|Default|GetWinScore))
          (CallFunction|PlayerStand)
          (return false)
          (else
            (return true)))))))